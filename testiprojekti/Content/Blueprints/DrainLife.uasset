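; DrainLife is a Blueprint effect that reduces the LifeForce of the player character passed to its ApplyEffect event.
; The amount removed is LifeDrain scaled by elapsed game time, so the drain grows the longer the game runs.
; LifeForce is floored at zero, and each application also sets the Blueprint's Speed variable to a fixed value.
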(event EventBeginPlay
  (|CallParentFunction) ; This node is disabled and will not be called.\nDrag off pins to build functionality.
)

(event Collision|EventActorBeginOverlap
  (params (OtherActor :type Actor%20Object%20Reference))
  (|CallParentFunction OtherActor) ; This node is disabled and will not be called.\nDrag off pins to build functionality.
)

(event EventTick
  (params (DeltaSeconds :type Float%20%28single-precision%29))
  (|CallParentFunction DeltaSeconds) ; This node is disabled and will not be called.\nDrag off pins to build functionality.
)

(event EventApplyEffect
  (params (Player%20Character :type BB%20My%20Character%20Object%20Reference))
  (if (> (- (Variables|/Game/Blueprints/BB_MyCharacter.BB_MyCharacter_C|GetlifeForce Player%20Character) (* (/ (Utilities|Time|GetGameTimeinSeconds) 5.0) (Variables|Default|GetLifeDrain))) 0.0)
    (Variables|/Game/Blueprints/BB_MyCharacter.BB_MyCharacter_C|SetlifeForce Player%20Character (- (Variables|/Game/Blueprints/BB_MyCharacter.BB_MyCharacter_C|GetlifeForce Player%20Character) (* (/ (Utilities|Time|GetGameTimeinSeconds) 5.0) (Variables|Default|GetLifeDrain))))
    (else
      (Variables|/Game/Blueprints/BB_MyCharacter.BB_MyCharacter_C|SetlifeForce Player%20Character 0.0)))
  (Variables|Default|SetSpeed 5e+02))

(fn ConstructionScript
  (|CallParentFunction))